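; Player controller that provides in-game text chat between players.
; On local BeginPlay it sets game-only input and adds a hidden chat panel widget, which Enter reveals and focuses.
; Submitted messages go through a server event that loops the GameState player array and calls each controller's client event to update its panel.
; Client events also restore game-only input when the chat box has focus and hide the panel on server request.
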(event Custom|Client_UpdateChat
  (params (PlayerName :type Text) (ChatMessage :type Text))
  (bind _chatpanel (Variables|Default|GetChatPanel)
    (:then
      (Default|UpdateChat _chatpanel PlayerName ChatMessage)
      (if (Class|Widget|HasKeyboardFocus (Variables|/Game/Blueprints/UI/WBP_ChatPanel.WBP_ChatPanel_C|GetChatInputBox (Variables|Default|GetChatPanel)))
        (Input|SetInputModeGameOnly self false)))
    (:else)))

(event Custom|Client_HideChat
  (Variables|/Script/UMG.Widget|SetVisibility (Variables|Default|GetChatPanel) "Hidden"))

(event Custom|Server_SubmitChat
  (params (PlayerName :type Text) (ChatMessage :type Text))
  (for _array_element (Variables|/Script/Engine.GameStateBase|GetPlayerArray (Game|GetGameState))
    (bind _asbp_player_controller (Utilities|Casting|CastToBP_PlayerController (Game|GetPlayerController _array_element)))
    (CallFunction|ClientUpdateChat _asbp_player_controller PlayerName ChatMessage)))

(event Custom|Server_HideChat
  (CallFunction|ClientHideChat))

(event EventBeginPlay
  (bind _returnvalue (Game|GetPlayerController 0))
  (if (Pawn|IsLocalController)
    (Utilities|IsValid _returnvalue
      (:Is%20Valid
        (Input|SetInputModeGameOnly _returnvalue false)
        (Variables|/Script/Engine.PlayerController|SetbShowMouseCursor _returnvalue false)
        (bind _returnvalue_2 (UserInterface|CreateWidget "/Game/Blueprints/UI/WBP_ChatPanel.WBP_ChatPanel_C" self))
        (bind _output_get (Variables|Default|SetChatPanel _returnvalue_2))
        (UserInterface|Viewport|AddtoViewport _output_get 0)
        (Widget|SetVisibility (Variables|Default|GetChatPanel) "Hidden")))))

(event Input|KeyboardEvents|Enter
  (params (Key :type Key%20Structure :default "None"))
  (:Pressed
    (if (not (Class|Widget|HasKeyboardFocus (Variables|/Game/Blueprints/UI/WBP_ChatPanel.WBP_ChatPanel_C|GetChatInputBox (Variables|Default|GetChatPanel))))
      (Widget|SetVisibility (Variables|Default|GetChatPanel) "Visible")
      (bind _chatpanel (Variables|Default|GetChatPanel)
        (:then
          (Widget|SetKeyboardFocus (Variables|/Game/Blueprints/UI/WBP_ChatPanel.WBP_ChatPanel_C|GetChatInputBox _chatpanel))
          (Default|HideChat (Variables|Default|GetChatPanel)))
        (:else)))))

(fn ConstructionScript)