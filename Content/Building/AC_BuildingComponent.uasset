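; Build-mode component for BP_ThirdPersonCharacter that previews and spawns pieces from the DT_Buildables table.
; While build mode is on, a self-re-arming Delay loop traces from the camera to position a ghost mesh.
; The ghost snaps to a hit actor's build boxes via interface messages, turning green on any hit, red otherwise.
; SpawnBuild spawns the selected actor at that transform and passes it the mesh, without checking CanBuild itself.
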(event Custom|BuildDelay
  (bind _buildghost (Variables|Default|GetBuildGhost))
  (if (Variables|Default|GetbIsBuildModeOn)
    (Utilities|FlowControl|Delay 0.01)
    (CallFunction|BuildCycle)
    (else
      (Variables|Default|SetbIsBuildModeOn false)
      (Variables|Default|SetbCanBuild false)
      (Utilities|IsValid _buildghost
        (:Is%20Valid
          (Default|DestroyComponent (Variables|Default|GetPlayerRef) _buildghost))))))

(event Custom|LaunchBuildMode
  (if (Variables|Default|GetbIsBuildModeOn)
    (CallFunction|StopBuildMode)
    (else
      (Variables|Default|SetbIsBuildModeOn true)
      (CallFunction|BuildCycle))))

(event Custom|StopBuildMode
  (bind _buildghost (Variables|Default|GetBuildGhost))
  (Variables|Default|SetbIsBuildModeOn false)
  (Variables|Default|SetbCanBuild false)
  (Utilities|IsValid _buildghost
    (:Is%20Valid
      (Default|DestroyComponent (Variables|Default|GetPlayerRef) _buildghost))))

(event EventBeginPlay
  (bind _asbp_third_person_character (Utilities|Casting|CastToBP_ThirdPersonCharacter (Components|GetOwner)))
  (Variables|Default|SetPlayerRef _asbp_third_person_character)
  (bind _outrownames (DataTable|GetDataTableRowNames "/Game/Building/DT_Buildables.DT_Buildables"))
  (for _array_element _outrownames
    (bind _returnvalue (Utilities|GetDataTableRow "/Game/Building/DT_Buildables.DT_Buildables" _array_element)
      (:then
        (Utilities|Array|Add (Variables|Default|GetBuildables) _returnvalue)))))

(fn SpawnBuildGhost
  (bind _returnvalue (Game|AddComponentbyClass (Variables|Default|GetPlayerRef) "/Script/Engine.StaticMeshComponent" false (Variables|Default|GetBuildTransform)))
  (bind _output_get (Variables|Default|SetBuildGhost _returnvalue))
  (Components|StaticMesh|SetStaticMesh _output_get (.mesh (Utilities|Array|Get(acopy) (Variables|Default|GetBuildables) (Variables|Default|GetBuildID))))
  (Collision|SetCollisionEnabled (Variables|Default|GetBuildGhost) "NoCollision"))

(fn GiveBuildColor
  (params (IsGreen :type Boolean))
  (bind _buildghost (Variables|Default|GetBuildGhost))
  (bind _output_get (Variables|Default|SetbCanBuild IsGreen))
  (for _index (range 0 (Rendering|Material|GetNumMaterials (Variables|Default|GetBuildGhost)))
    (if _output_get
      (Rendering|Material|SetMaterial _buildghost _index "/Game/Building/Materials/M_GreenColor.M_GreenColor")
      (else
        (Rendering|Material|SetMaterial _buildghost _index "/Game/Building/Materials/M_RedColor.M_RedColor"))))
  (Transformation|SetWorldTransform (Variables|Default|GetBuildGhost) (Variables|Default|GetBuildTransform) false false))

(fn BuildCycle
  (bind _camera (Variables|Default|GetCamera))
  (bind _buildghost (Variables|Default|GetBuildGhost))
  (bind _returnvalue (Math|Vector|GetForwardVector _camera))
  (bind _returnvalue_2 (Transformation|GetWorldLocation _camera))
  (bind (_outhit _returnvalue_3) (Collision|LineTraceByChannel (+ _returnvalue_2 (* _returnvalue 350)) (+ _returnvalue_2 (* _returnvalue 1500)) (.tracechannel (Utilities|Array|Get(acopy) (Variables|Default|GetBuildables) (Variables|Default|GetBuildID))) false 0 "None"))
  (if _returnvalue_3
    (Variables|Default|SetBuildTransform (Math|Transform|MakeTransform (.ImpactPoint (Collision|BreakHitResult _outhit)) (.rotation (Variables|Default|GetBuildTransform)) (.scale (Variables|Default|GetBuildTransform))))
    (Variables|Default|SetHit%20Actor (.HitActor (Collision|BreakHitResult _outhit)))
    (Variables|Default|SetHit%20Component (.HitComponent (Collision|BreakHitResult _outhit)))
    (Utilities|IsValid _buildghost
      (:Is%20Valid
        (bind (_found _transform) (CallFunction|DetectBuildBoxes))
        (if _found
          (Variables|Default|SetBuildTransform _transform))
        (CallFunction|GiveBuildColor true)
        (CallFunction|BuildDelay))
      (:Is%20Not%20Valid
        (CallFunction|SpawnBuildGhost :!label _label)
        (CallFunction|BuildDelay :!label _label_2)))
    (else
      (Variables|Default|SetBuildTransform (Math|Transform|MakeTransform (.TraceEnd (Collision|BreakHitResult _outhit)) (.rotation (Variables|Default|GetBuildTransform)) (.scale (Variables|Default|GetBuildTransform))))
      (Utilities|IsValid _buildghost
        (:Is%20Valid
          (CallFunction|GiveBuildColor false)
          (goto _label_2))
        (:Is%20Not%20Valid
          (goto _label))))))

(fn ChangeMesh
  (bind _buildghost (Variables|Default|GetBuildGhost))
  (Utilities|IsValid _buildghost
    (:Is%20Valid
      (Components|StaticMesh|SetStaticMesh _buildghost (.mesh (Utilities|Array|Get(acopy) (Variables|Default|GetBuildables) (Variables|Default|GetBuildID)))))))

(fn SpawnBuild
  (bind _returnvalue (Game|SpawnActorfromClass (.actor (Utilities|Array|Get(acopy) (Variables|Default|GetBuildables) (Variables|Default|GetBuildID))) (Variables|Default|GetBuildTransform) "Undefined" "MultiplyWithRoot" 0 0))
  (Class|BuildInterface|SetMesh(Message) _returnvalue (.mesh (Utilities|Array|Get(acopy) (Variables|Default|GetBuildables) (Variables|Default|GetBuildID)))))

(fn DetectBuildBoxes
  (bind _boxes (Class|BuildInterface|ReturnBoxes(Message) (Variables|Default|GetHit%20Actor)))
  (bind _array_element (Utilities|Array|ForEachLoopwithBreak _boxes :!label _label)
    (:LoopBody
      (if (== (Variables|Default|GetHit%20Component) _array_element)
        (LocalVariables|SetLocalFound true)
        (goto _label Break)))
    (:Completed
      (return (LocalVariables|GetLocalFound) (Transformation|GetWorldTransform (Variables|Default|GetHit%20Component))))))